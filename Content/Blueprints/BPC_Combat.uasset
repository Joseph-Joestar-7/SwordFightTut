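; Player combat component for BP_ThirdPersonCharacter, handling target lock, directional dodge and sword combo attacks.
; Lock-on sphere-traces for a pawn, attaches a marker, and steers control rotation toward it each tick.
; Dodge and attack montages spend stamina and pause its regen; montage notifies continue the combo if input was buffered, otherwise stop it.
; TraceDamage starts a looping timer that sphere-traces between sword points, applying DoOnce-throttled damage and sound.
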(event Custom|Event%20Trace%20Damage
  ;[0.2535 0.2535 0.2535] Sword Traces
  (bind _returnvalue (Utilities|Time|SetTimerbyEvent (delegate Custom|Damage%20Trace) 0.01 true)))

(event Custom|Damage%20Trace
  (bind _playerbp (Variables|Default|GetPlayerBP))
  ;[0.2535 0.2535 0.2535] Sword Traces
  (bind (_outhit _returnvalue) (Collision|SphereTraceForObjects (Transformation|GetWorldLocation (Variables|/Game/ThirdPerson/Blueprints/BP_ThirdPersonCharacter.BP_ThirdPersonCharacter_C|GetStart%20Sword%20Trace%20Pos _playerbp)) (Transformation|GetWorldLocation (Variables|/Game/ThirdPerson/Blueprints/BP_ThirdPersonCharacter.BP_ThirdPersonCharacter_C|GetEnd%20Sword%20Trace%20Pos _playerbp)) 25.0 (Utilities|Array|MakeArray "ObjectTypeQuery3") false 0 "ForOneFrame"))
  (if _returnvalue
    (Utilities|FlowControl|DoOnce false :!label _label
      (:Completed
        (Game|Damage|ApplyDamage (.HitActor (Collision|BreakHitResult _outhit)) (Variables|Default|GetswordDamage) 0 0)
        (Audio|PlaySoundatLocation "/Game/Audio/Sounds/MS_Damage.MS_Damage" (.Location (Collision|BreakHitResult _outhit)) "0, 0, 0" 1.0 1.0 0.0 0 0 0 0)
        (Utilities|FlowControl|Delay 0.3)
        (goto _label Reset)))))

(event Custom|End%20Damage%20Trace
  ;[0.2535 0.2535 0.2535] Sword Traces
  (if (Utilities|Time|IsValidTimerHandle (stale Custom|Event%20Trace%20Damage _returnvalue))
    (Utilities|Time|ClearandInvalidateTimerbyHandle (stale Custom|Event%20Trace%20Damage _returnvalue))))

(event Input|EnhancedActionEvents|EnhancedInputActionIA_Lock
  (params (ActionValue :type Boolean) (ElapsedSeconds :type Float%20%28double-precision%29) (TriggeredSeconds :type Float%20%28double-precision%29) (InputAction :type Input%20Action%20Object%20Reference :default "/Game/ThirdPerson/Input/Actions/IA_Lock.IA_Lock"))
  (bind _returnvalue (Game|GetPlayerCameraManager 0))
  (bind _playerbp (Variables|Default|GetPlayerBP))
  (bind _playerbp_2 (Variables|Default|GetPlayerBP))
  (bind _charactermovement (Variables|/Script/Engine.Character|GetCharacterMovement _playerbp))
  (bind _rootcomponent (Variables|/Script/Engine.Actor|GetRootComponent _returnvalue))
  (bind _charactermovement_2 (Variables|/Script/Engine.Character|GetCharacterMovement _playerbp_2))
  (bind _returnvalue_2 (Transformation|GetWorldLocation _rootcomponent))
  (:Started
    (Variables|Default|GetTargetLockActor
      (:then
        (Variables|Default|SetTargetLockActor 0)
        (Variables|/Script/Engine.CharacterMovementComponent|SetbOrientRotationToMovement _charactermovement true)
        (Variables|/Script/Engine.CharacterMovementComponent|SetbUseControllerDesiredRotation _charactermovement false)
        (Actor|DestroyActor (Variables|Default|GetTargetLockWidget)))
      (:else
        (bind (_outhit _returnvalue_3) (Collision|SphereTraceForObjects "0, 0, 0" (+ (Math|Vector|MakeVector (.x _returnvalue_2) (.y _returnvalue_2) (+ (.z _returnvalue_2) 2e+01)) (* (Math|Vector|GetForwardVector (Transformation|GetWorldRotation _rootcomponent)) 1e+03)) 1.5e+02 (Utilities|Array|MakeArray "ObjectTypeQuery3") false 0 "ForDuration" true "(R=1.000000,G=0.000000,B=0.000000,A=1.000000)" "(R=0.000000,G=1.000000,B=0.000000,A=1.000000)" 2.0))
        (if _returnvalue_3
          (Variables|Default|SetTargetLockActor (.HitActor (Collision|BreakHitResult _outhit)))
          (Variables|/Script/Engine.CharacterMovementComponent|SetbOrientRotationToMovement _charactermovement_2 false)
          (Variables|/Script/Engine.CharacterMovementComponent|SetbUseControllerDesiredRotation _charactermovement_2 true)
          (bind _returnvalue_4 (Game|SpawnActorfromClass "/Game/Blueprints/BP_TargetLockWidget.BP_TargetLockWidget_C" (Math|Transform|MakeTransform (Math|Vector|MakeVector (.x (.location (Transformation|GetActorTransform (Variables|Default|GetTargetLockActor)))) (.y (.location (Transformation|GetActorTransform (Variables|Default|GetTargetLockActor)))) (+ (.z (.location (Transformation|GetActorTransform (Variables|Default|GetTargetLockActor)))) 2e+01)) (.rotation (Transformation|GetActorTransform (Variables|Default|GetTargetLockActor))) "1.000000,1.000000,1.000000") "AlwaysSpawn" "MultiplyWithRoot" 0 0))
          (bind _output_get (Variables|Default|SetTargetLockWidget _returnvalue_4))
          (Transformation|AttachActorToActor _output_get (Variables|Default|GetTargetLockActor) "None" "SnapToTarget" "SnapToTarget" "SnapToTarget" true))))))

(event Input|EnhancedActionEvents|EnhancedInputActionIA_Attack
  (params (ActionValue :type Boolean) (ElapsedSeconds :type Float%20%28double-precision%29) (TriggeredSeconds :type Float%20%28double-precision%29) (InputAction :type Input%20Action%20Object%20Reference :default "/Game/ThirdPerson/Input/Actions/IA_Attack.IA_Attack"))
  (bind _playerbp (Variables|Default|GetPlayerBP))
  (bind _bpc_stats (Variables|/Game/ThirdPerson/Blueprints/BP_ThirdPersonCharacter.BP_ThirdPersonCharacter_C|GetBPC_Stats _playerbp))
  ;[0.2535 0.2535 0.2535] Sword Combo Animation
  (:Started
    (if (Math|Boolean|ANDBoolean (not (Variables|Default|GetisAttacking)) (>= (Variables|/Game/Blueprints/BPC_Stats.BPC_Stats_C|GetStamina (Variables|/Game/ThirdPerson/Blueprints/BP_ThirdPersonCharacter.BP_ThirdPersonCharacter_C|GetBPC_Stats (Variables|Default|GetPlayerBP))) 1e+01) (Variables|/Game/ThirdPerson/Blueprints/BP_ThirdPersonCharacter.BP_ThirdPersonCharacter_C|GetisWeaponEquipped? (Variables|Default|GetPlayerBP)))
      (Variables|Default|SetisAttacking true)
      (Animation|Montage|PlayMontage (Variables|/Script/Engine.Character|GetMesh (Variables|Default|GetPlayerBP)) "/Game/Characters/Souls/Combat/SwordAttackCombo_Montage.SwordAttackCombo_Montage"
        (:then
          (Variables|/Game/Blueprints/BPC_Stats.BPC_Stats_C|SetregainStamina? _bpc_stats false)
          (Default|IncreaseValue _bpc_stats "NewEnumerator1" -1e+01 :!label _label))
        (:OnCompleted
          (Variables|Default|SetisAttacking false :!label _label_2)
          (Variables|Default|Setcombo false)
          (Variables|/Game/Blueprints/BPC_Stats.BPC_Stats_C|SetregainStamina? (Variables|/Game/ThirdPerson/Blueprints/BP_ThirdPersonCharacter.BP_ThirdPersonCharacter_C|GetBPC_Stats (Variables|Default|GetPlayerBP)) true))
        (:OnInterrupted
          (goto _label_2))
        (:OnNotifyBegin
          (if (and (Variables|Default|GetisAttacking) (Variables|Default|Getcombo))
            (Variables|Default|Setcombo false)
            (goto _label)
            (else
              (Animation|Montage|MontageStop (Components|SkeletalMesh|GetAnimInstance (Variables|/Script/Engine.Character|GetMesh (Variables|Default|GetPlayerBP))) 0.2 "/Game/Characters/Souls/Combat/SwordAttackCombo_Montage.SwordAttackCombo_Montage")))))
      (else
        (Variables|Default|Setcombo true)))))

(event Input|EnhancedActionEvents|EnhancedInputActionIA_Dodge
  (params (ActionValue :type Boolean) (ElapsedSeconds :type Float%20%28double-precision%29) (TriggeredSeconds :type Float%20%28double-precision%29) (InputAction :type Input%20Action%20Object%20Reference :default "/Game/ThirdPerson/Input/Actions/IA_Dodge.IA_Dodge"))
  (bind _playerbp (Variables|Default|GetPlayerBP))
  (bind _bpc_stats (Variables|/Game/ThirdPerson/Blueprints/BP_ThirdPersonCharacter.BP_ThirdPersonCharacter_C|GetBPC_Stats _playerbp))
  (:Started
    (if (and (not (Variables|Default|GetisDodging)) (>= (Variables|/Game/Blueprints/BPC_Stats.BPC_Stats_C|GetStamina (Variables|/Game/ThirdPerson/Blueprints/BP_ThirdPersonCharacter.BP_ThirdPersonCharacter_C|GetBPC_Stats (Variables|Default|GetPlayerBP))) 5.0))
      (Variables|Default|SetisDodging true)
      (Utilities|FlowControl|Sequence
        (:then_0
          (if true
            (switch string (Utilities|String|ToString(Text) (Class|KismetInputLibrary|KeyGetDisplayName (Variables|/Game/ThirdPerson/Blueprints/BP_ThirdPersonCharacter.BP_ThirdPersonCharacter_C|GetDirection%20Key (Variables|Default|GetPlayerBP)) true))
              (:W
                (Variables|Default|SetmovementDirection "NewEnumerator0"))
              (:A
                (Variables|Default|SetmovementDirection "NewEnumerator1"))
              (:S
                (Variables|Default|SetmovementDirection "NewEnumerator2"))
              (:D
                (Variables|Default|SetmovementDirection "NewEnumerator3")))
            (else
              (Variables|Default|SetmovementDirection "NewEnumerator0"))))
        (:then_1
          (Animation|Montage|PlayMontage (Variables|/Script/Engine.Character|GetMesh (Variables|Default|GetPlayerBP)) (Utilities|Select :Index (Variables|Default|GetmovementDirection) :NewEnumerator0 "/Game/Characters/Souls/Combat/Dodge/Dodge_F_Montage.Dodge_F_Montage" :NewEnumerator1 "/Game/Characters/Souls/Combat/Dodge/Dodge_L_Montage.Dodge_L_Montage" :NewEnumerator2 "/Game/Characters/Souls/Combat/Dodge/Dodge_B_Montage.Dodge_B_Montage" :NewEnumerator3 "/Game/Characters/Souls/Combat/Dodge/Dodge_R_Montage.Dodge_R_Montage")
            (:then
              (Variables|/Game/Blueprints/BPC_Stats.BPC_Stats_C|SetregainStamina? _bpc_stats false)
              (Default|IncreaseValue _bpc_stats "NewEnumerator1" -5.0))
            (:OnCompleted
              (Variables|Default|SetisDodging false :!label _label)
              (Variables|/Game/Blueprints/BPC_Stats.BPC_Stats_C|SetregainStamina? (Variables|/Game/ThirdPerson/Blueprints/BP_ThirdPersonCharacter.BP_ThirdPersonCharacter_C|GetBPC_Stats (Variables|Default|GetPlayerBP)) true))
            (:OnInterrupted
              (goto _label))))))))

(event EventTick
  (params (DeltaSeconds :type Float%20%28single-precision%29))
  (bind _playerbp (Variables|Default|GetPlayerBP))
  (bind _targetlockactor (Variables|Default|GetTargetLockActor))
  (bind _returnvalue (Transformation|GetActorLocation _targetlockactor))
  (bind _returnvalue_2 (Transformation|GetActorLocation _playerbp))
  (bind _returnvalue_3 (Math|Rotator|FindLookatRotation _returnvalue_2 _returnvalue))
  ;[0.2535 0.2535 0.2535] Target Lock Update
  (Variables|Default|GetTargetLockActor
    (:then
      (Pawn|SetControlRotation (Pawn|GetController (Variables|Default|GetPlayerBP)) (Math|Rotator|MakeRotator (.roll _returnvalue_3) (+ (.pitch _returnvalue_3) -2e+01) (.yaw _returnvalue_3))))
    (:else)))

(event EventBeginPlay
  ;[0.2535 0.2535 0.2535] Get Player Class
  (bind _asbp_third_person_character (Utilities|Casting|CastToBP_ThirdPersonCharacter (Components|GetOwner)))
  (Variables|Default|SetPlayerBP _asbp_third_person_character))