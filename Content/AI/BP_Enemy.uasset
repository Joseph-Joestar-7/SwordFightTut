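; BP_Enemy is a melee enemy, with a boss variant, that attacks with montages and dies into a ragdoll before being destroyed.
; BPCStats handles incoming damage and drives the overhead health bar widget.
; A looping timer runs sword or boss-punch sphere traces between begin and end events, with a DoOnce and delay limiting repeat hits.
; A separate point trace deals fixed area damage with sound and camera shake.
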(event Custom|Damage%20Trace
  (bind _isboss (Variables|Default|GetisBoss))
  ;[0.2535 0.2535 0.2535] Sword Traces
  (if (not (Variables|Default|GetisDead?))
    (bind (_outhit _returnvalue) (Collision|SphereTraceForObjects (Math|Vector|SelectVector (Variables|Default|GetstartBossPunchTrace) (Transformation|GetWorldLocation (Variables|Default|GetStart%20Sword%20Trace%20Pos)) _isboss) (Math|Vector|SelectVector (Variables|Default|GetendBossPunchTrace) (Transformation|GetWorldLocation (Variables|Default|GetEnd%20Sword%20Trace%20Pos)) _isboss) (Variables|Default|GetAttackRadius) (Utilities|Array|MakeArray "ObjectTypeQuery3") false 0 "ForOneFrame"))
    (if _returnvalue
      (Utilities|FlowControl|DoOnce false :!label _label
        (:Completed
          (Game|Damage|ApplyDamage (.HitActor (Collision|BreakHitResult _outhit)) (Variables|Default|GetswordDamage) 0 0)
          (Utilities|FlowControl|Delay 0.3)
          (goto _label Reset))))))

(event EventBeginPlay
  (bind _aswb_enemy_health (Utilities|Casting|CastToWB_EnemyHealth (UserInterface|GetWidget (Variables|Default|GetWidget))))
  (Default|SetHealthProgressBar (Variables|Default|GetBPC_Stats) (Variables|/Game/UI/WB_EnemyHealth.WB_EnemyHealth_C|GetHealthBar _aswb_enemy_health)))

(event Collision|EventActorBeginOverlap
  (params (OtherActor :type Actor%20Object%20Reference)))

(event EventTick
  (params (DeltaSeconds :type Float%20%28single-precision%29)))

(event EventBeginSwordTrace
  ;[0.2535 0.2535 0.2535] Sword Traces
  (bind _returnvalue (Utilities|Time|SetTimerbyEvent (delegate Custom|Damage%20Trace) 0.01 true)))

(event EventEndSwordTrace
  ;[0.2535 0.2535 0.2535] Sword Traces
  (if (Utilities|Time|IsValidTimerHandle (stale EventBeginSwordTrace _returnvalue))
    (Utilities|Time|ClearandInvalidateTimerbyHandle (stale EventBeginSwordTrace _returnvalue))))

(event Game|Damage|EventAnyDamage
  (params (Damage :type Float%20%28single-precision%29) (DamageType :type Damage%20Type%20Object%20Reference) (InstigatedBy :type Controller%20Object%20Reference) (DamageCauser :type Actor%20Object%20Reference))
  (Default|IncreaseValue (Variables|Default|GetBPC_Stats) "NewEnumerator0" (* Damage -1.0)))

(event EventDie
  (Pawn|Components|CharacterMovement|DisableMovement (Variables|Character|GetCharacterMovement))
  (Physics|SetSimulatePhysics (Variables|Character|GetMesh) true)
  (Variables|Default|SetisDead? true)
  (Utilities|FlowControl|Delay 4.0)
  (Actor|DestroyActor))

(event EventPointDamageTrace
  (bind _point_damage_pos (Variables|Default|GetPoint%20Damage%20Pos))
  (bind _returnvalue (Transformation|GetWorldLocation _point_damage_pos))
  (Utilities|FlowControl|Sequence
    (:then_0
      (bind (_outhit _returnvalue_2) (Collision|SphereTraceForObjects _returnvalue _returnvalue (Variables|Default|GetPointDamageRadius) (Utilities|Array|MakeArray "ObjectTypeQuery3") false 0 "None"))
      (if _returnvalue_2
        (Game|Damage|ApplyDamage (.HitActor (Collision|BreakHitResult _outhit)) 1e+01 0 0)
        (Audio|PlaySoundatLocation "/Game/Audio/Sounds/Thump.Thump" (.Location (Collision|BreakHitResult _outhit)) "0, 0, 0" 1.0 1.0 0.0 0 0 0 0)
        (Camera|PlayWorldCameraShake "/Game/Blueprints/BP_CameraShake_Attack.BP_CameraShake_Attack_C" (.Location (Collision|BreakHitResult _outhit)) 0.0 2e+03)))))

(fn ConstructionScript)

(fn BigAttack
  (bind _returnvalue (Animation|PlayAnimMontage (Variables|Default|GetAnim%20Montage_0) 1.0 "None"))
  (Audio|PlaySoundatLocation "/Game/Audio/Sounds/SC_Thrall.SC_Thrall" (Transformation|GetActorLocation) "0, 0, 0" 1.0 1.0 0.0 0 0 0 0)
  (return _returnvalue))

(fn SwordAttack
  (bind _returnvalue (Animation|PlayAnimMontage (Variables|Default|GetAnim%20Montage) 1.0 "None"))
  (Audio|PlaySoundatLocation "/Game/Audio/Sounds/SC_Thrall.SC_Thrall" (Transformation|GetActorLocation) "0, 0, 0" 1.0 1.0 0.0 0 0 0 0)
  (return _returnvalue))